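; Stealth-game enemy AI character that patrols, investigates noises and chases the player on sight, sending them back to a checkpoint with a melee hit.
; Tick picks chase, patrol-point looping or random roaming from PlayerVisible and CanMove, with AIMoveTo handling movement.
; PawnSensing drives detection, and a retriggerable delay clears sightings.
; The attack montage's notify triggers a hand-socket sphere trace, while JumptoDestination launches the enemy along a projectile arc.
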(event OnSeePawn(PawnSensing)
  (params (Pawn :type Pawn%20Object%20Reference))
  ;[0.15 0.15 0.15 0.5] Determines whether the player is spotted/visible
  (Utilities|FlowControl|Sequence
    (:then_0
      (Utilities|Casting|CastToBP_ThirdPersonCharacterCustom Pawn
        (:then
          (Development|PrintString "Stop right there!")
          (Variables|Default|SetbPlayerVisible true))
        (:CastFailed
          (Variables|Default|SetbPlayerVisible false))))
    (:then_1
      (Utilities|FlowControl|RetriggerableDelay 3.0)
      (Development|PrintString "Must've been the wind.")
      (Variables|Default|SetbPlayerVisible false))))

(event OnHearNoise(PawnSensing)
  (params (Instigator :type Pawn%20Object%20Reference) (Location :type Vector%20%28by%20ref%29 :default "0, 0, 0") (Volume :type Float%20%28single-precision%29))
  (CallFunction|UpdateWalkSpeed 2e+02)
  (Variables|Default|SetbCanMove false)
  (AI|AIMoveTo self Location Instigator 5.0 false
    (:OnSuccess
      _)
    (:OnFail
      _))
  (Utilities|FlowControl|Delay 8.0)
  (Variables|Default|SetbCanMove true))

(event Custom|ChasePlayer
  ;[0.15 0.15 0.15 0.5] Chases the player when they are spotted
  (CallFunction|UpdateWalkSpeed 4e+02)
  (Variables|Default|SetbCanMove false)
  (AI|AIMoveTo self "0, 0, 0" (Game|GetPlayerCharacter 0) 5e+01 false
    (:OnSuccess
      (CallFunction|Attack)
      (Utilities|FlowControl|Delay 2.0)
      (Variables|Default|SetbCanMove true))))

(event Custom|Attack
  (bind _mesh (Variables|Character|GetMesh))
  (bind _returnvalue (Transformation|GetSocketLocation _mesh "hand_r"))
  ;[0.15 0.1407 0.04319 0.5] Bonk
  (Utilities|FlowControl|DoOnce false ; Only Reset Attack on miss.
    (:Completed
      (bind _notifyname (Animation|Montage|PlayMontage (Variables|Character|GetMesh) "/Game/StealthGame/Characters/Enemies/AM_Attack_01.AM_Attack_01") ; Play the AM_Attack_01
        (:then
          (CallFunction|ResetAttack))
        (:OnNotifyBegin
          (switch name _notifyname ; Pick the proper attack type(standard when there is more than one type of attack)
            (:AttackDamage
              (Development|PrintString "I'm attacking!")
              (bind (_outhits _returnvalue_2) (Collision|MultiSphereTraceForObjects _returnvalue (+ _returnvalue (* (Transformation|GetActorForwardVector) (Variables|Default|GetMeleeTraceDistance))) (Variables|Default|GetMeleeTraceRadius) (Utilities|Array|MakeArray "ObjectTypeQuery3") false 0 "None")) ; Trace forward from hand socket.
              (if _returnvalue_2 ; If a pawn is hit in that trace...
                (for _array_element _outhits ; ...loop through the results....
                  (bind _asbp_third_person_character_custom (Utilities|Casting|CastToBP_ThirdPersonCharacterCustom (.HitActor (Collision|BreakHitResult _array_element))))
                  (Default|LoadCheckpoint _asbp_third_person_character_custom))))))))))

(event Custom|MoveToNextPatrolPoint
  ;[0.15 0.15 0.15 0.5] Tells the AI to patrol to specific points
  (CallFunction|UpdateWalkSpeed 2e+02)
  (Variables|Default|SetbCanMove false)
  (AI|AIMoveTo self "0, 0, 0" (Utilities|Array|Get(acopy) (Variables|Default|GetPatrolTargetPoints) (Variables|Default|GetPatrolTargetPointIndex)) 8e+01 false
    (:OnSuccess
      (Utilities|FlowControl|Delay 3.0)
      (Variables|Default|SetbCanMove true)
      (CallFunction|SetNextPatrolPointIndex))))

(event Custom|ResetAttack
  (bind _mesh (Variables|Character|GetMesh))
  (bind _returnvalue (Transformation|GetSocketLocation _mesh "hand_r"))
  ;[0.15 0.1407 0.04319 0.5] Bonk
  (Utilities|FlowControl|DoOnce false) ; enters at Reset
)

(event Custom|PatrolRandom
  ;[0.15 0.15 0.15 0.5] Patrols random points in a radius
  (CallFunction|UpdateWalkSpeed 2e+02)
  (Variables|Default|SetbCanMove false)
  (AI|AIMoveTo self (.RandomLocation (AI|Navigation|GetRandomReachablePointinRadius (Transformation|GetActorLocation) 2e+03 0 0)) 0 8e+01 false
    (:OnSuccess
      _)
    (:OnFail
      _))
  (Utilities|FlowControl|Delay 3.0)
  (Variables|Default|SetbCanMove true))

(event Custom|SetNextPatrolPointIndex
  ;[0.15 0.15 0.15 0.5] Tells the Patrol Point array to advance one, and repeat after end is reached
  (Variables|Default|SetPatrolTargetPointIndex (Math|Integer|%(Integer) (+ (Variables|Default|GetPatrolTargetPointIndex) 1) (Utilities|Array|Length (Variables|Default|GetPatrolTargetPoints)))))

(event EventBeginPlay
  ;[0.15 0.15 0.15 0.5] Begins AI patrol cycle on play
  (CallFunction|PatrolRandom))

(event EventJumptoDestination
  (params (Destination :type Vector :default "0, 0, 0"))
  (bind (_x _y _z) (Math|Vector|BreakVector Destination))
  ;[0.15 0.15 0.15 0.5] The AI will jump to follow the player when reaching relevant points on the map
  (bind _outlaunchvelocity (Game|SuggestProjectileVelocityCustomArc (Transformation|GetActorLocation) (Math|Vector|MakeVector _x _y (+ _z 2.5e+02)) 0.0 0.5))
  (Character|LaunchCharacter _outlaunchvelocity true true))

(event EventTick
  (params (DeltaSeconds :type Float%20%28single-precision%29))
  (bind _bplayervisible (Variables|Default|GetbPlayerVisible))
  ;[0.15 0.15 0.15 0.5] Determines whether the AI should be patrolling or chasing
  (if (Variables|Default|GetbCanMove)
    (if _bplayervisible
      (CallFunction|ChasePlayer)
      (elif (Variables|Default|GetbTargetPointMovement)
        (CallFunction|MovetoNextPatrolPoint)
        (else
          (CallFunction|PatrolRandom))))
    (elif _bplayervisible
      (CallFunction|ChasePlayer))))

(fn ConstructionScript)

(fn UpdateWalkSpeed
  (params (NewWalkSpeed :type Float%20%28double-precision%29))
  (Variables|/Script/Engine.CharacterMovementComponent|SetMaxWalkSpeed (Variables|Character|GetCharacterMovement) NewWalkSpeed))