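; Trap door interactable that slides open when the player character overlaps it, then closes again.
; An overlap with BP_ThirdPersonCharacterCustom prints a debug message and plays an opening timeline that lerps the Cube's relative X location.
; The opening timeline's Update, rather than Finished, feeds a two-second Delay that starts a second timeline in reverse from its end to slide the Cube back.
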(event EventBeginPlay)

(event EventTick
  (params (DeltaSeconds :type Float%20%28single-precision%29)))

(event Collision|EventActorBeginOverlap
  (params (OtherActor :type Actor%20Object%20Reference))
  (Utilities|Casting|CastToBP_ThirdPersonCharacterCustom OtherActor)
  (Development|PrintString "The player is here!!")
  (bind _newtrack_0 (Timeline|OpeningTrapDoor Play) ; Timeline for opening
    (:Update
      (Transformation|SetRelativeLocation (Variables|Default|GetCube) (Math|Vector|MakeVector (Math|Float|Lerp 0.0 -1e+03 _newtrack_0) 0.0 0.0) false false)
      (Utilities|FlowControl|Delay 2.0)
      (bind _newtrack_0_2 (Timeline|Timeline ReverseFromEnd) ; Timeline for closing
        (:Update
          (Transformation|SetRelativeLocation (Variables|Default|GetCube) (Math|Vector|MakeVector (Math|Float|Lerp 0.0 -1e+03 _newtrack_0_2) 0.0 0.0) false false))))))

(fn ConstructionScript)